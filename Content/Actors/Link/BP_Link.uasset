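; Player-controlled Link in a Zelda-style game, with movement, a sword attack and a heart-meter HUD created on BeginPlay.
; Movement axes set a four-way Direction and swap Link's directional material, polling with a short Delay until any active sword is gone.
; Attack plays a sound and spawns BP_Sword at that direction's spawn point.
; The sword flies at full health; otherwise it attaches there, unless existing attached swords are found and destroyed.
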(event `InputAxis|MoveForward`
  (params (AxisValue :type "Float (single-precision)"))
  ;[1 1 1] Movement input handler
  (`self.AddMovementInput` (`KismetMathLibrary.GetForwardVector` (`KismetMathLibrary.MakeRotator` 0.0 (.pitch (`self.GetControlRotation`)))) AxisValue)
  (`/Engine/EditorBlueprintResources/StandardMacros.CompareFloat` AxisValue
    (:`>`
      (if (not (`|EnumEquality` (`self.Direction`) "NewEnumerator0"))
        (set `self.Direction` "NewEnumerator0")
        ;[1 1 1] Update material with specific direction
        (set `self.Directional Material` "/Game/Actors/Link/WalkSprites/M_link_north.M_link_north")
        (if (`KismetSystemLibrary.IsValid` (`self.Swinging Sword`)) :!label _label
          ;[1 1 1] Sloppy, find better solution.
          ; Animations?
          (`KismetSystemLibrary.Delay` 0.016667)
          (goto _label)
          (else
            (`PrimitiveComponent.SetMaterial` (`self.Link`) 0 (`self.Directional Material`))))))
    (:`<`
      (if (not (`|EnumEquality` (`self.Direction`) "NewEnumerator2"))
        (set `self.Direction` "NewEnumerator2")
        (set `self.Directional Material` "/Game/Actors/Link/WalkSprites/M_link_south.M_link_south")
        (goto _label)))))

(event `InputAxis|MoveRight`
  (params (AxisValue :type "Float (single-precision)"))
  ;[1 1 1] Movement input handler
  (`self.AddMovementInput` (`KismetMathLibrary.GetRightVector` (`KismetMathLibrary.MakeRotator` 0.0 (.pitch (`self.GetControlRotation`)))) AxisValue)
  (`/Engine/EditorBlueprintResources/StandardMacros.CompareFloat` AxisValue
    (:`>`
      (if (not (`|EnumEquality` (`self.Direction`) "NewEnumerator1"))
        (set `self.Direction` "NewEnumerator1")
        ;[1 1 1] Update material with specific direction
        (set `self.Directional Material` "/Game/Actors/Link/WalkSprites/M_link_east.M_link_east")
        (goto _label)))
    (:`<`
      (if (not (`|EnumEquality` (`self.Direction`) "NewEnumerator3"))
        (set `self.Direction` "NewEnumerator3")
        (set `self.Directional Material` "/Game/Actors/Link/WalkSprites/M_link_west.M_link_west")
        (goto _label)))))

(event `InputAction|Attack`
  (params (Key :type "Key Structure"))
  ;[1 1 1] Attack input handler
  (:`Pressed`
    (`self.Summon Sword` (== (`self.Health`) (`self.Max Health`)))))

(event `self.ReceiveBeginPlay`
  ;[1 1 1] Create HUD
  (bind _returnvalue (`|CreateWidget` "/Game/Actors/Link/HUDSprites/W_heart_meter.W_heart_meter_C"))
  (bind _output_get (set `self.Heart Meter` _returnvalue))
  (set `/Game/Actors/Link/HUDSprites/W_heart_meter.Health` (`self.Health`) _output_get)
  (set `/Game/Actors/Link/HUDSprites/W_heart_meter.Max Health` (`self.Max Health`) _output_get)
  (`UserWidget.AddToViewport` _output_get 0)
  (set `PlayerController.bShowMouseCursor` false (`GameplayStatics.GetPlayerController` 0)))

(fn `Summon Sword`
  (params (Flying :type Boolean))
  (locals (`Summoned Swords` :type "Array of /Game/Actors/Weapons/Sword/BP_Sword Object Reference") (NewLocalVar_0 :type "SceneComponent Object Reference"))
  (bind _swinging_sword (`self.Swinging Sword`))
  (bind _returnvalue (select `/Game/Utils/CardinalDirections` (`self.Direction`) :`NewEnumerator0` (`self.Sword Spawnpoint North`) :`NewEnumerator1` (`self.Sword Spawnpoint East`) :`NewEnumerator2` (`self.Sword Spawnpoint South`) :`NewEnumerator3` (`self.Sword Spawnpoint West`)))
  ;[1 1 1] Initial condition testing
  (`/Engine/EditorBlueprintResources/StandardMacros.IsValid` _swinging_sword
    (:`Is Valid`
      (if (`self.Destroy Old Sword`)
        (`self.K2_DestroyActor` _swinging_sword)
        ;[1 1 1] Play sound
        (`GameplayStatics.PlaySoundAtLocation` "/Game/Audio/LinkAttack.LinkAttack" (`SceneComponent.K2_GetComponentLocation` (`self.Camera`)) (struct) 1.0 1.0 0.0 null null null :!label _label)
        ;[1 1 1] Summon sword
        (bind _returnvalue_2 (`|SpawnActorFromClass` "/Game/Actors/Weapons/Sword/BP_Sword.BP_Sword_C" (`KismetMathLibrary.MakeTransform` (`SceneComponent.K2_GetComponentLocation` _returnvalue)) "Undefined" "OverrideRootScale" self self))
        (bind _output_get (set `self.Swinging Sword` _returnvalue_2))
        (if Flying
          (`/Game/Actors/Weapons/Sword/BP_Sword.Fly` _output_get)
          (else
            ;;[1 1 1] Find if a sword is attached, and delete existing ones
            (bind _filteredarray (`KismetArrayLibrary.FilterArray` (`self.GetAttachedActors` false) "/Game/Actors/Weapons/Sword/BP_Sword.BP_Sword_C"))
            (`/Engine/EditorBlueprintResources/StandardMacros.CompareInt` (`KismetArrayLibrary.Array_Length` _filteredarray)
              (:`>`
                (for _array_element _filteredarray
                  (`self.K2_DestroyActor` _array_element)))
              (:`==`
                (`SceneComponent.K2_AttachToComponent` (`Actor.RootComponent` _output_get) _returnvalue "None" "SnapToTarget" "KeepWorld" "KeepRelative" true)))))))
    (:`Is Not Valid`
      (goto _label))))

(fn `UserConstructionScript`)