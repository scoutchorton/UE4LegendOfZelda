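; BP_Sword is a sword weapon actor that either performs a timed swing or, once Fly is called, travels along world Y.
; Tick drives both modes with swept movement: the swing snaps Root to -90 yaw, rotates to 90 over RotationDuration, then destroys the actor.
; Hitbox end-overlap events record each actor once in Hitlist and only print debug text, with no damage applied.
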(event `self.Hitbox.OnComponentEndOverlap`
  (params (OverlappedComponent :type "PrimitiveComponent Object Reference") (OtherActor :type "Actor Object Reference") (OtherComp :type "PrimitiveComponent Object Reference") (OtherBodyIndex :type Integer))
  (bind _hitlist (`self.Hitlist`))
  ;[1 1 1] Collision handling
  (if (not (`KismetArrayLibrary.Array_Contains` _hitlist OtherActor))
    (`KismetArrayLibrary.Array_Add` _hitlist OtherActor)
    (`|ExecutionSequence`
      (:`then_0`
        (`KismetSystemLibrary.PrintString` "OVERLAP"))
      (:`then_1`
        (`KismetSystemLibrary.PrintString` (`KismetSystemLibrary.GetDisplayName` OtherActor))))))

(event `self.ReceiveTick`
  (params (DeltaSeconds :type "Float (single-precision)"))
  (bind _root (`self.Root`))
  ;[1 1 1] Initial flying testing
  (if (`self.Flying`)
    ;[1 1 1] Flying sword handling
    (`self.K2_AddActorWorldOffset` (`KismetMathLibrary.MakeVector` 0.0 (* DeltaSeconds (`self.Fly Speed`))) true)
    (else
      ;[1 1 1] Not flying sword
      (if (`self.Sweeping`)
        ;;[1 1 1] Normal swinging action
        (`SceneComponent.K2_AddRelativeRotation` _root (`KismetMathLibrary.MakeRotator` 0.0 0.0 (* DeltaSeconds (/ 180.0 (`self.Rotation Duration`)))) true false)
        (`/Engine/EditorBlueprintResources/StandardMacros.CompareFloat` (.yaw (.rotation (`SceneComponent.GetRelativeTransform` _root))) 90.0
          (:`>`
            _)
          (:`==`
            _))
        (`self.K2_DestroyActor`)
        (set `self.Sweeping` false)
        (`KismetArrayLibrary.Array_Clear` (`self.Hitlist`))
        (else
          ;;[1 1 1] Sword setup
          (`SceneComponent.K2_SetRelativeRotation` _root (`KismetMathLibrary.MakeRotator` 0.0 0.0 -90.0) false true)
          (set `self.Sweeping` true))))))

(fn `Fly`
  (set `self.Flying` true))

(fn `UserConstructionScript`)